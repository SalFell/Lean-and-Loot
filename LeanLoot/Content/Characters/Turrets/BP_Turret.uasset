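; Turret that fires BP_TurretProjectile from its Arrow in timed bursts separated by cooldowns, starting at BeginPlay if Active.
; A looping timer drives Shoot, while a second timer triggers Cooldown, which clears firing and restarts the cycle after a delay.
; Overlap with BP_StunGunProjectile halts firing and attaches sparks until a retriggerable stun delay ends.
; SetActive toggles Active; switching off leaves running timers untouched, and GetActive always returns false.
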(event `/Game/Characters/Turrets/BPI_Turret.SetActive`
  (params (`Active?` :type Boolean))
  (bind _active (`self.Active`))
  ;[1 1 1 0.5] Interface to allow toggling 'Active' variable
  (bind _output_get (set `self.Active` `Active?`))
  (if _output_get
    ;[1 1 1] Standard Shooting/Cooldown Logic
    (if _active :!label _label
      ;;[0 0.15 0.003098 0.5] Shoot at specified firerate
      (bind _returnvalue (`KismetSystemLibrary.K2_SetTimerDelegate` (delegate `Shoot`) (`self.Firerate`) _active))
      (set `self.ShootTimer` _returnvalue)
      ;;[0 0.15 0.00593 0.5] After shooting for specified time, go Cooldown
      (`KismetSystemLibrary.K2_SetTimerDelegate` (delegate `Cooldown`) (`self.ShootingTime`)))))

(event `self.ReceiveBeginPlay`
  ;[1 1 1] Standard Shooting/Cooldown Logic
  (goto _label))

(event `Cooldown`
  (bind _shoottimer (`self.ShootTimer`))
  ;[1 1 1] Standard Shooting/Cooldown Logic
  ;;[0 0.15 0.00593 0.5] After shooting for specified time, go Cooldown
  (`KismetSystemLibrary.K2_PauseTimerHandle` _shoottimer)
  (`KismetSystemLibrary.K2_ClearAndInvalidateTimerHandle` _shoottimer)
  (`KismetSystemLibrary.Delay` (`self.CooldownTime`))
  (goto _label))

(event `Shoot`
  (bind _arrow (`self.Arrow`))
  ;[1 1 1] Standard Shooting/Cooldown Logic
  ;;[0 0.15 0.003098 0.5] Shoot at specified firerate
  (`|SpawnActorFromClass` "/Game/Characters/Turrets/BP_TurretProjectile.BP_TurretProjectile_C" (`SceneComponent.K2_GetComponentToWorld` _arrow) "Undefined" "OverrideRootScale" self null)
  (`GameplayStatics.PlaySoundAtLocation` "/Game/FPWeapon/Audio/FirstPersonTemplateWeaponFire02.FirstPersonTemplateWeaponFire02" (`SceneComponent.K2_GetComponentLocation` _arrow) (struct) 0.1 1.0 0.0 null null null null) ; Play firing sound
)

(event `self.Capsule.OnComponentBeginOverlap`
  (params (OverlappedComponent :type "PrimitiveComponent Object Reference") (OtherActor :type "Actor Object Reference") (OtherComp :type "PrimitiveComponent Object Reference") (OtherBodyIndex :type Integer) (bFromSweep :type Boolean) (SweepResult :type "HitResult Structure (by ref)"))
  (bind _staticmesh (`self.StaticMesh`))
  (bind _shoottimer (`self.ShootTimer`))
  ;[0 0.15 0.003098 0.5] Stunning Logic. Stops turret shooting when hit by a stun projectile for a specified time
  (if (`GameplayStatics.ObjectIsA` OtherActor "/Game/FirstPerson/Blueprints/BP_StunGunProjectile.BP_StunGunProjectile_C")
    (set `self.Active` false)
    (`KismetSystemLibrary.K2_PauseTimerHandle` _shoottimer)
    (`KismetSystemLibrary.K2_ClearAndInvalidateTimerHandle` _shoottimer)
    (if (`KismetSystemLibrary.IsValid` (`self.EmitterHandle`))
      (`ActorComponent.K2_DestroyComponent` (`self.EmitterHandle`)))
    (bind _returnvalue (`GameplayStatics.SpawnEmitterAttached` "/Game/StarterContent/Particles/P_Sparks.P_Sparks" _staticmesh (`SceneComponent.GetAttachSocketName` _staticmesh) (0.0 0.0 0.0) (struct) (`SceneComponent.K2_GetComponentScale` _staticmesh) "SnapToTarget"))
    (bind _output_get (set `self.EmitterHandle` _returnvalue))
    (`KismetSystemLibrary.RetriggerableDelay` (`self.StunTime`))
    (set `self.Active` true)
    (`ActorComponent.K2_DestroyComponent` _output_get)
    (goto _label)))

(fn `GetActive`
  (returns (Active :type Boolean))
  (return false))

(fn `UserConstructionScript`)